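; Triggerable elevator that alternates between two positions, Pos1 and Pos2, and carries a list of attached actors with it.
; Trigger flips the target only while idle, and Tick eases the mesh toward it with VInterpTo until nearly there.
; SetElevatorLocation moves attached actors by offsets cached at BeginPlay, quitting the game on an array length mismatch.
; The mesh location is stored for saving and reapplied at BeginPlay.
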(event EventBeginPlay
  (Utilities|Array|Clear (Variables|Default|GetRelativeLocations))
  (for _array_element (Variables|Default|GetAttachedActors)
    (Utilities|Array|Add (Variables|Default|GetRelativeLocations) (- (Transformation|GetActorLocation _array_element) (Transformation|GetWorldLocation (Variables|Default|GetElevatorMesh))))
    (CallFunction|SetElevatorLocation (Variables|Default|GetSavedElevatorLocation))))

(event Collision|EventActorBeginOverlap
  (params (OtherActor :type Actor%20Object%20Reference)))

(event EventTick
  (params (DeltaSeconds :type Float%20%28single-precision%29))
  (bind _elevatormesh (Variables|Default|GetElevatorMesh))
  (bind _target (Variables|Default|GetTarget))
  (bind _relativelocation (Variables|/Script/Engine.SceneComponent|GetRelativeLocation _elevatormesh))
  (bind _returnvalue (Math|Interpolation|VInterpTo _relativelocation _target DeltaSeconds 2.0))
  (if (not (Variables|Default|GetbIsIdling))
    (CallFunction|SetElevatorLocation _returnvalue)
    (Variables|Default|SetbIsIdling (Math|Vector|VectorIsNearlyZero (- _returnvalue (Variables|Default|GetTarget)) 1.0))))

(event EventTrigger
  (if (Variables|Default|GetbIsIdling)
    (if (Variables|Default|GetbForward)
      (Variables|Default|SetTarget (Variables|/Script/Engine.SceneComponent|GetRelativeLocation (Variables|Default|GetPos1)))
      (else
        (Variables|Default|SetTarget (Variables|/Script/Engine.SceneComponent|GetRelativeLocation (Variables|Default|GetPos2)))))
    (Variables|Default|SetbForward (not (Variables|Default|GetbForward)))
    (Variables|Default|SetbIsIdling false)))

(fn ConstructionScript)

(fn SetElevatorLocation
  (params (Relative%20location :type Vector))
  (bind _relativelocations (Variables|Default|GetRelativeLocations))
  (bind _returnvalue (Utilities|Array|Length _relativelocations))
  (Transformation|SetRelativeLocation (Variables|Default|GetElevatorMesh) Relative%20location false false)
  (if (!= (Utilities|Array|Length (Variables|Default|GetAttachedActors)) _returnvalue)
    (Class|VisualLoggerKismetLibrary|LogText 0 "Error! Lengths must be equal" "VisLogBP")
    (Game|QuitGame 0 "Quit" false)
    (else
      (for _index (range 0 (- _returnvalue 1))
        (Transformation|SetActorLocation (Utilities|Array|Get(acopy) (Variables|Default|GetAttachedActors) _index) (+ (Transformation|GetWorldLocation (Variables|Default|GetElevatorMesh)) (Utilities|Array|Get(acopy) (Variables|Default|GetRelativeLocations) _index)) false false)))))

(fn GetActorSaveData
  (Variables|Default|SetSavedElevatorLocation (Variables|/Script/Engine.SceneComponent|GetRelativeLocation (Variables|Default|GetElevatorMesh)))
  (bind _returnvalue (|CallParentFunction))
  (return _returnvalue))

(fn CanbeTriggered
  (return (Variables|Default|GetbIsIdling)))
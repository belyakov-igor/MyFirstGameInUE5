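; Interaction helper component that makes its owning InteractableActor glow while it has focus.
; On BeginPlay it binds to the owner's focus-in and focus-out events and creates a dynamic material instance from slot 0 of the owner's static mesh.
; Focus in sets that material's Emissive Power parameter to the configured EmissivePower value, and focus out resets it to zero.
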(event Custom|FocusOut
  (Rendering|Material|SetScalarParameterValue (Variables|Default|GetMaterialInstance) "Emissive Power" 0.0 :!class /Script/Engine.MaterialInstanceDynamic))

(event Custom|FocusIn
  (Rendering|Material|SetScalarParameterValue (Variables|Default|GetMaterialInstance) "Emissive Power" (Variables|Focus|GetEmissivePower) :!class /Script/Engine.MaterialInstanceDynamic))

(event EventBeginPlay
  (bind _asinteractable_actor (Utilities|Casting|CastToInteractableActor (Components|GetOwner)))
  (EventDispatchers|BindEventtoFocusin _asinteractable_actor (delegate Custom|FocusIn))
  (EventDispatchers|BindEventtoFocusOut _asinteractable_actor (delegate Custom|FocusOut))
  (bind _returnvalue (Rendering|Material|CreateDynamicMaterialInstance (Actor|GetComponentbyClass _asinteractable_actor "/Script/Engine.StaticMeshComponent") 0 (Rendering|Material|GetMaterial (Actor|GetComponentbyClass _asinteractable_actor "/Script/Engine.StaticMeshComponent") 0) "None" :!class /Script/Engine.PrimitiveComponent))
  (Variables|Default|SetMaterialInstance _returnvalue))

(event EventTick
  (params (DeltaSeconds :type Float%20%28single-precision%29)))
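; BP_Button is an interactable push button that calls Trigger on a linked Triggerable when pressed.
; Interact starts a press if idle, and Tick eases the mesh along local X to a target displacement and back with FInterpTo.
; The trigger fires as the press reaches full depth.
; Each tick, IsEnabled combines the idle state with the target's CanBeTriggered message, and FocusText supplies the focus prompt.
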(event EventBeginPlay
  (Variables|Default|SetBackupMeshLocation (Variables|/Script/Engine.SceneComponent|GetRelativeLocation (Variables|Default|GetStaticMesh))))

(event Collision|EventActorBeginOverlap
  (params (OtherActor :type Actor%20Object%20Reference)))

(event EventTick
  (params (DeltaSeconds :type Float%20%28single-precision%29))
  (bind _backupmeshlocation (Variables|Default|GetBackupMeshLocation))
  (Utilities|FlowControl|Sequence
    (:then_0
      (bind _returnvalue (Class|Triggerable|CanbeTriggered(Message) (Variables|Interaction|GetTriggerable)))
      (Variables|Default|SetbIsEnabled (and (Variables|Default|GetbIsIdling) _returnvalue)))
    (:then_1
      (if (not (Variables|Default|GetbIsIdling))
        (Variables|Default|SetCurrentDisplacement (Math|Interpolation|FInterpTo (Variables|Default|GetCurrentDisplacement) (select (Variables|Default|GetbForward) (Variables|Interaction|GetTargetDisplacement) 0.0) DeltaSeconds 6.0))
        (Transformation|SetRelativeLocation (Variables|Default|GetStaticMesh) (Math|Vector|MakeVector (+ (Variables|Default|GetCurrentDisplacement) (.x _backupmeshlocation)) (.y _backupmeshlocation) (.z _backupmeshlocation)) false false)
        (Utilities|FlowControl|Sequence
          (:then_0
            (if (and (Math|Float|NearlyEqual(Float) (Variables|Default|GetCurrentDisplacement) (Variables|Interaction|GetTargetDisplacement) 0.2) (Variables|Default|GetbForward))
              (Variables|Default|SetbForward false)
              (bind _astriggerable (Utilities|Casting|CastToTriggerable (Variables|Interaction|GetTriggerable)))
              (Class|Triggerable|Trigger _astriggerable)))
          (:then_1
            (if (and (Math|Float|NearlyEqual(Float) (Variables|Default|GetCurrentDisplacement) 0.0 0.2) (not (Variables|Default|GetbForward)))
              (Variables|Default|SetbIsIdling true))))))))

(event EventInteract
  (params (Pawn :type Pawn%20Object%20Reference))
  (|CallParentFunction 0)
  (if (Variables|Default|GetbIsIdling)
    (Variables|Default|SetbIsIdling false)
    (Variables|Default|SetbForward true)))

(fn ConstructionScript)

(fn FocusText
  (return (Variables|Interaction|GetFocusTextValue)))
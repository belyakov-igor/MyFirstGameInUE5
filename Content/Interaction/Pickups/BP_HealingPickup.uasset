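; BP_HealingPickup is a healing pickup actor that glows while it has interaction focus; no healing logic is defined in these graphs.
; The Construction Script creates a dynamic material instance from the mesh's first material slot.
; Focus-in and focus-out events call their parent versions, then raise or clear that instance's Emissive Power parameter to toggle the highlight.
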(event EventBeginPlay)

(event Collision|EventActorBeginOverlap
  (params (OtherActor :type Actor%20Object%20Reference)))

(event EventTick
  (params (DeltaSeconds :type Float%20%28single-precision%29)))

(event EventFocusin
  (|CallParentFunction)
  (Rendering|Material|SetScalarParameterValue (Variables|Default|GetMaterialInstance) "Emissive Power" 0.3 :!class /Script/Engine.MaterialInstanceDynamic))

(event EventFocusOut
  (|CallParentFunction)
  (Rendering|Material|SetScalarParameterValue (Variables|Default|GetMaterialInstance) "Emissive Power" 0.0 :!class /Script/Engine.MaterialInstanceDynamic))

(fn ConstructionScript
  (bind _mesh (Variables|Character|GetMesh))
  (bind _returnvalue (Rendering|Material|CreateDynamicMaterialInstance _mesh 0 (Rendering|Material|GetMaterial _mesh 0) "None" :!class /Script/Engine.PrimitiveComponent))
  (Variables|Default|SetMaterialInstance _returnvalue))
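; Weapon pickup Blueprint that represents a selectable weapon in the world and highlights when focused.
; The construction script uses WeaponID to index parallel arrays for class, name, ammo amount and mesh, then creates a dynamic material instance on that mesh.
; Focus in and out events call their parent versions, then switch the material's Emissive Power glow on or off.
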(event EventBeginPlay)

(event Collision|EventActorBeginOverlap
  (params (OtherActor :type Actor%20Object%20Reference)))

(event EventTick
  (params (DeltaSeconds :type Float%20%28single-precision%29)))

(event EventFocusin
  (|CallParentFunction)
  (Rendering|Material|SetScalarParameterValue (Variables|Default|GetMaterialInstance) "Emissive Power" 0.3 :!class /Script/Engine.MaterialInstanceDynamic))

(event EventFocusOut
  (|CallParentFunction)
  (Rendering|Material|SetScalarParameterValue (Variables|Default|GetMaterialInstance) "Emissive Power" 0.0 :!class /Script/Engine.MaterialInstanceDynamic))

(fn ConstructionScript
  (bind _mesh (Variables|Character|GetMesh))
  ;[0 0.09759 0.2016 0.302] Set Pickup Variables
  (Variables|Default|SetWeaponClass (Utilities|Array|Get(acopy) (Variables|Default|GetWeaponClasses) (Variables|Pickup|GetWeaponID)))
  (Variables|Default|SetWeaponName (Utilities|Array|Get(acopy) (Variables|Default|GetWeaponNames) (Variables|Pickup|GetWeaponID)))
  (Variables|Default|SetAmmoAmount (Utilities|Array|Get(acopy) (Variables|Default|GetAmmoAmounts) (Variables|Pickup|GetWeaponID)))
  ;[0 0.09759 0.2016 0.302] Mesh and material
  (Components|StaticMesh|SetStaticMesh (Variables|Character|GetMesh) (Utilities|Array|Get(acopy) (Variables|Default|GetMeshes) (Variables|Pickup|GetWeaponID)))
  (bind _returnvalue (Rendering|Material|CreateDynamicMaterialInstance _mesh 0 (Rendering|Material|GetMaterial _mesh 0) "None" :!class /Script/Engine.PrimitiveComponent))
  (Variables|Default|SetMaterialInstance _returnvalue))